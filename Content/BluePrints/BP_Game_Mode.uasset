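; Game mode for a space shooter that tracks score, kills and difficulty level and relays player death to the HUD.
; PlayerDead calls PlayerKapoot on BP_SpaceShoot_HUD, fetched from the first player controller.
; ExtractPoints adds enemy score to Progress once the HUD cast succeeds.
; EnemyDestroyed counts kills and raises Level on every second one.
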(event Custom|PlayerDead
  (bind _asbp_space_shoot_hud (Utilities|Casting|CastToBP_SpaceShoot_HUD (HUD|GetHUD (Game|GetPlayerController 0))))
  (Default|PlayerKapoot _asbp_space_shoot_hud))

(event Custom|ExtractPoints
  (params (score :type Float%20%28double-precision%29))
  ;[1 1 1] Update Score After Enmey Dead
  (Utilities|Casting|CastToBP_SpaceShoot_HUD (HUD|GetHUD (Game|GetPlayerController 0)))
  (Variables|Default|SetProgress (+ (Variables|Default|GetProgress) score)))

(event Custom|EnemyDestroyed
  (bind _output_get (Variables|Default|SetEnemiesDestroyed (+ (Variables|Default|GetEnemiesDestroyed) 1)))
  (if (== (Math|Integer|%(Integer) _output_get 2) 0)
    (Variables|Default|SetLevel (+ (Variables|Default|GetLevel) 1))))

(event EventBeginPlay)

(event EventTick
  (params (DeltaSeconds :type Float%20%28single-precision%29)))

(fn ConstructionScript)