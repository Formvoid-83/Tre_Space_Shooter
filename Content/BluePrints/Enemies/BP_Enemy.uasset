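; BP_Enemy is an enemy actor that moves along a movement vector and fires ammo at regular intervals.
; Tick offsets its location by speed and delta time, and accumulates a timer that spawns Ammo at FireSpawn with the enemy's rotation.
; Overlaps destroy it after short delays: player contact broadcasts OnEnemyDestroy, blocking volumes remove it silently, and player ammo passes ScoreValue to the game mode's ExtractPoints.
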(event Custom|Destroyed_Event
  (Utilities|FlowControl|Delay 0.1)
  (Actor|DestroyActor))

(event EventBeginPlay
  (EventDispatchers|BindEventtoOnEnemyDestroy (delegate Custom|Destroyed_Event)))

(event Collision|EventActorBeginOverlap
  (params (OtherActor :type Actor%20Object%20Reference))
  (bind _tags (Variables|/Script/Engine.Actor|GetTags OtherActor))
  (if (Utilities|Array|ContainsItem _tags "Player")
    ;[1 1 1] Collision with Player
    (Default|CallOnEnemyDestroy)
    (Utilities|Casting|CastToBP_Game_Mode (Game|GetGameMode))
    (Audio|PlaySound2D "/Game/Assets/Sound/S_HIt.S_HIt" 1.0 1.0 0.0 0 0)
    (Utilities|FlowControl|Delay 0.2)
    (Actor|DestroyActor)
    (else
      ;[1 1 1] Collision with Limit
      (if (Utilities|Array|ContainsItem _tags "BLOCK")
        (Utilities|Casting|CastToBlockingVolume OtherActor)
        (Utilities|FlowControl|Delay 0.2)
        (Actor|DestroyActor)
        (else
          ;[1 1 1] Player shoots Us
          (Utilities|Casting|CastToBP_Player_Ammo OtherActor)
          (bind _asbp_game_mode (Utilities|Casting|CastToBP_Game_Mode (Game|GetGameMode)))
          (Default|ExtractPoints _asbp_game_mode (Variables|Default|GetscoreValue))
          (Audio|PlaySound2D "/Game/Assets/Sound/S_HIt.S_HIt" 1.0 1.0 0.0 0 0)
          (Utilities|FlowControl|Delay 0.2)
          (Actor|DestroyActor))))))

(event EventTick
  (params (DeltaSeconds :type Float%20%28single-precision%29))
  ;[1 1 1] Move
  (CallFunction|Move DeltaSeconds)
  (bind _output_get (Variables|Default|SetShotCurrentTime (+ DeltaSeconds (Variables|Default|GetShotCurrentTime))))
  ;[1 1 1] Shoot
  (if (> _output_get (Variables|Default|GetDelayShot))
    (Variables|Default|SetShotCurrentTime 0.0)
    (CallFunction|Fire)))

(fn ConstructionScript)

(fn Move
  (params (DeltaTime :type Float%20%28double-precision%29))
  (Transformation|SetActorLocation (+ (Transformation|GetActorLocation) (* (* DeltaTime (Variables|Default|GetSpeed)) (Variables|Default|GetMovementVector))) false false))

(fn Fire
  (bind _returnvalue (Game|SpawnActorfromClass (Variables|Default|GetAmmo) (Transformation|GetWorldTransform (Variables|Default|GetFireSpawn)) "Undefined" "MultiplyWithRoot" 0 0))
  (Transformation|SetActorRotation _returnvalue (Transformation|GetActorRotation)))