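; Player ship pawn for a 2D-style shooter that moves, fires and loses lives when hit.
; Enhanced Input drives movement clamped to fixed X/Y bounds and timer-throttled firing of BP_Player_Ammo.
; Tag-based overlaps cost lives from enemies and bullets unless ShieldActive, notifying BP_Game_Mode at zero.
; Shield pickups show a timed shield sprite, though this graph never sets ShieldActive to true.
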(event Custom|EnableFire
  ;[1 1 1] Shooting
  (Variables|Default|SetCanFire true))

(event Custom|DamageActor
  ;[1 1 1] Recive Damage
  (Audio|PlaySound2D "/Game/Effects/bad_beeps_4.bad_beeps_4" 1.0 1.0 0.0 0 0)
  (bind _output_get (Variables|Default|SetLives (- (Variables|Default|GetLives) 1)))
  (if (== _output_get 0)
    (bind _asbp_game_mode (Utilities|Casting|CastToBP_Game_Mode (Game|GetGameMode)))
    (Default|PlayerDead _asbp_game_mode)))

(event Custom|StopShield
  ;[1 1 1] Use Shield Item
  (Variables|Default|SetshieldActive false)
  (Rendering|SetVisibility (Variables|Default|GetSpriteShield) false false))

(event Input|EnhancedActionEvents|EnhancedInputActionIA_MoveRight
  (params (ActionValue :type Float%20%28double-precision%29) (ElapsedSeconds :type Float%20%28double-precision%29) (TriggeredSeconds :type Float%20%28double-precision%29) (InputAction :type Input%20Action%20Object%20Reference :default "/Game/Inputs/Actions/IA_MoveRight.IA_MoveRight"))
  (bind _returnvalue (Transformation|GetActorLocation))
  (bind (_x _y _z) (Math|Vector|BreakVector _returnvalue))
  ;[1 1 1] Movement
  (Pawn|Input|AddMovementInput "1.000000,0.000000,0.000000" ActionValue false)
  (Transformation|SetActorLocation self (Math|Vector|MakeVector (Math|Float|Clamp(Float) _x -43.0 1445.0) (Math|Float|Clamp(Float) _y -863.0 -39.0) _z) false false))

(event Input|EnhancedActionEvents|EnhancedInputActionIA_UpDown
  (params (ActionValue :type Float%20%28double-precision%29) (ElapsedSeconds :type Float%20%28double-precision%29) (TriggeredSeconds :type Float%20%28double-precision%29) (InputAction :type Input%20Action%20Object%20Reference :default "/Game/Inputs/Actions/IA_UpDown.IA_UpDown"))
  (bind _returnvalue (Transformation|GetActorLocation))
  (bind (_x _y _z) (Math|Vector|BreakVector _returnvalue))
  ;[1 1 1] Movement
  (Pawn|Input|AddMovementInput "0.000000,1.000000,0.000000" ActionValue false)
  (Transformation|SetActorLocation self (Math|Vector|MakeVector (Math|Float|Clamp(Float) _x -43.0 1445.0) (Math|Float|Clamp(Float) _y -863.0 -39.0) _z) false false))

(event Input|EnhancedActionEvents|EnhancedInputActionIA_Shoot
  (params (ActionValue :type Boolean) (ElapsedSeconds :type Float%20%28double-precision%29) (TriggeredSeconds :type Float%20%28double-precision%29) (InputAction :type Input%20Action%20Object%20Reference :default "/Game/Inputs/Actions/IA_Shoot.IA_Shoot"))
  ;[1 1 1] Shooting
  (if (Variables|Default|GetCanFire)
    (CallFunction|DoFire)
    (Variables|Default|SetCanFire false)
    (Utilities|Time|SetTimerbyEvent (delegate Custom|EnableFire) (Variables|Default|GetFireDelay))))

(event EventBeginPlay
  ;[1 1 1] Setting Up Movement by Input
  (bind _asplayer_controller (Utilities|Casting|CastToPlayerController (Pawn|GetController)))
  (Input|AddMappingContext (PlayerController|LocalPlayerSubsystems|GetEnhancedInputLocalPlayerSubsystem _asplayer_controller) "/Game/Inputs/IMC_ShipMovement.IMC_ShipMovement" 0 "(bIgnoreAllPressedKeysUntilRelease=True,bForceImmediately=False,bNotifyUserSettings=False)"))

(event Collision|EventActorBeginOverlap
  (params (OtherActor :type Actor%20Object%20Reference))
  ;[1 1 1] Use Shield Item
  (if (Utilities|Array|ContainsItem (Variables|/Script/Engine.Actor|GetTags OtherActor) "ShieldPowerUp")
    (if (Utilities|IsValid OtherActor)
      (Audio|PlaySound2D "/Game/Effects/pick_up_3.pick_up_3" 1.0 1.0 0.0 0 0)
      (Rendering|SetVisibility (Variables|Default|GetSpriteShield) true false)
      (Utilities|Time|SetTimerbyEvent (delegate Custom|StopShield) (Variables|Default|GetshieldDuration)))
    (elif (Utilities|Array|ContainsItem (Variables|/Script/Engine.Actor|GetTags OtherActor) "Enemy")
      (if (not (Variables|Default|GetshieldActive))
        (Utilities|Casting|CastToBP_Enemy OtherActor)
        (CallFunction|DamageActor))
      (elif (Utilities|Array|ContainsItem (Variables|/Script/Engine.Actor|GetTags OtherActor) "EBullet")
        (if (not (Variables|Default|GetshieldActive))
          ;[1 1 1] Got Shot
          (CallFunction|DamageActor))))))

(event EventTick
  (params (DeltaSeconds :type Float%20%28single-precision%29)))

(fn ConstructionScript)

(fn DoFire
  (Game|SpawnActorfromClass "/Game/BluePrints/BP_Player_Ammo.BP_Player_Ammo_C" (Transformation|GetWorldTransform (Variables|Default|GetFireSpwan)) "Undefined" "MultiplyWithRoot" 0 0)
  (Audio|PlaySound2D "/Game/Effects/low_beep.low_beep" 1.0 1.0 0.0 0 0))