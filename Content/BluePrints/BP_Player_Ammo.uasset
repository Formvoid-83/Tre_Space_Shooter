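; BP_Player_Ammo is the player's projectile, which moves along its local Y axis each tick at its Speed without sweeping.
; On overlapping an actor tagged Enemy that casts to BP_Enemy, or otherwise a BlockingVolume, it plays a hit sound and destroys itself after a short delay.
; It applies no damage to the enemy itself, and BeginPlay only prints its spawn height.
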(event EventBeginPlay
  ;[1 1 1] Start of Spawn
  (Development|PrintString (Utilities|String|ToString(Float) (.Z (Math|Vector|BreakVector (Transformation|GetActorLocation)))) true true "(R=1.000000,G=0.849252,B=0.020833,A=1.000000)"))

(event Collision|EventActorBeginOverlap
  (params (OtherActor :type Actor%20Object%20Reference))
  (if (Utilities|Array|ContainsItem (Variables|/Script/Engine.Actor|GetTags OtherActor) "Enemy")
    ;[1 1 1] Collide with Enemy
    (Utilities|Casting|CastToBP_Enemy OtherActor)
    (Audio|PlaySound2D "/Game/Assets/Sound/S_HIt.S_HIt" 1.0 1.0 0.0 0 0)
    (Utilities|FlowControl|Delay 0.2)
    (Actor|DestroyActor)
    (else
      ;[1 1 1] Collide with Limit
      (Utilities|Casting|CastToBlockingVolume OtherActor)
      (Audio|PlaySound2D "/Game/Assets/Sound/S_HIt.S_HIt" 1.0 1.0 0.0 0 0)
      (Utilities|FlowControl|Delay 0.2)
      (Actor|DestroyActor))))

(event EventTick
  (params (DeltaSeconds :type Float%20%28single-precision%29))
  ;[1 1 1] Shot movement
  (Transformation|AddActorLocalOffset (Math|Vector|MakeVector 0.0 (* DeltaSeconds (Variables|Default|GetSpeed)) 0.0) false false))

(fn ConstructionScript)