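; Random item generator actor that periodically spawns shield pickups (BP_ItemShield) in the level.
; BeginPlay starts a looping timer at SpawnTime and caches the BP_Game_Mode reference, which is not otherwise used here.
; Each tick of that timer calls SpawnShield, placing a shield at a random XY within hardcoded bounds at fixed height.
; RefreshTime resets the SpawnTime variable but does not restart the running timer.
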(event Custom|SpawnItem
  (CallFunction|SpawnShield))

(event Custom|RefreshTime
  (Variables|Default|SetSpawnTime 15.0))

(event EventBeginPlay
  (Utilities|Time|SetTimerbyEvent (delegate Custom|SpawnItem) (Variables|Default|GetSpawnTime) true)
  (bind _asbp_game_mode (Utilities|Casting|CastToBP_Game_Mode (Game|GetGameMode)))
  (Variables|Default|Setm_Game_Mode _asbp_game_mode))

(event Collision|EventActorBeginOverlap
  (params (OtherActor :type Actor%20Object%20Reference)))

(event EventTick
  (params (DeltaSeconds :type Float%20%28single-precision%29)))

(fn ConstructionScript)

(fn SpawnShield
  (bind _returnvalue (Game|SpawnActorfromClass "/Game/BluePrints/Items/BP_ItemShield.BP_ItemShield_C" (Math|Transform|MakeTransform (Math|Vector|MakeVector (Math|Random|RandomFloatinRange 4e+01 1.37e+03) (Math|Random|RandomFloatinRange -7.8e+02 -1.4e+02) -44.558232)) "AdjustIfPossibleButAlwaysSpawn" "MultiplyWithRoot" 0 0))
  (return _returnvalue))