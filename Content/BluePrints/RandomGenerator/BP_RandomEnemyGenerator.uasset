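; BP_RandomEnemyGenerator is an actor that spawns a random enemy on a looping timer at one of its SpawnPoint-tagged scene components.
; The game mode's Level sets the random range for the enemy type, which is clamped and mapped to BP_Enemy or BP_Enemy2, with a third slot empty.
; Each spawned enemy's destroy event lowers SpawnTime, but the timer set at BeginPlay is never restarted with the new value.
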(event Custom|Spawn
  (bind _asbp_enemy (CallFunction|SpawnEnemy))
  (bind _asbp_enemy_2 (Utilities|Casting|CastToBP_Enemy _asbp_enemy))
  (EventDispatchers|BindEventtoOnEnemyDestroy _asbp_enemy_2 (delegate Custom|EnemyDestroyed)))

(event Custom|EnemyDestroyed
  (Variables|Default|SetSpawnTime (- (Variables|Default|GetSpawnTime) 1.0)))

(event EventBeginPlay
  (Utilities|Time|SetTimerbyEvent (delegate Custom|Spawn) (Variables|Default|GetSpawnTime) true)
  (bind _asbp_game_mode (Utilities|Casting|CastToBP_Game_Mode (Game|GetGameMode)))
  (Variables|Default|Setm_Game_Mode _asbp_game_mode))

(event Collision|EventActorBeginOverlap
  (params (OtherActor :type Actor%20Object%20Reference)))

(event EventTick
  (params (DeltaSeconds :type Float%20%28single-precision%29)))

(fn ConstructionScript)

(fn SpawnEnemy
  (bind _returnvalue (Actor|GetComponentsbyTag "/Script/Engine.SceneComponent" "SpawnPoint"))
  (bind _returnvalue_2 (CallFunction|GetClasstoSpawn (Math|Random|RandomInteger (Variables|/Game/BluePrints/BP_Game_Mode.BP_Game_Mode_C|GetLevel (Variables|Default|Getm_Game_Mode)))))
  (bind _returnvalue_3 (Game|SpawnActorfromClass _returnvalue_2 (Transformation|GetWorldTransform (Utilities|Array|Get(acopy) _returnvalue (Math|Random|RandomInteger (Utilities|Array|Length _returnvalue)))) "AdjustIfPossibleButAlwaysSpawn" "MultiplyWithRoot" 0 0))
  (return _returnvalue_3))

(fn GetClasstoSpawn
  (params (Type :type Integer))
  (return (Utilities|Select :Index (Math|Integer|Clamp(Integer) Type 0 (- (Variables|Default|GetMaxNumenemies) 1)) :Option%200 "/Game/BluePrints/Enemies/BP_Enemy.BP_Enemy_C" :Option%201 "/Game/BluePrints/Enemies/BP_Enemy2.BP_Enemy2_C" :Option%202 0)))